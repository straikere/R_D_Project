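; BP_PillarFollower is an actor that shuttles back and forth between the player's character and a pillar, with a randomly colored arrow set at spawn.
; Each Tick it eases toward its current target with VInterpTo, rotates to face it, and flips the MoveToCharacter flag once within range.
; Movement pauses while it is close to both targets at once, preventing jitter when the character stands by the pillar.
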(event EventBeginPlay
  ;[1 1 1] При створенні робить фоловера случайного кольору
  (Components|Arrow|SetArrowColor(LinearColor) (Variables|Default|GetArrow) (Math|Color|MakeColor (Math|Random|RandomFloat) (Math|Random|RandomFloat) (Math|Random|RandomFloat))))

(event EventTick
  (params (DeltaSeconds :type Float%20%28single-precision%29))
  (bind _returnvalue (Transformation|GetActorLocation))
  (bind _returnvalue_2 (Transformation|GetActorLocation))
  (bind _returnvalue_3 (Transformation|GetActorLocation))
  (bind _returnvalue_4 (Transformation|GetActorLocation))
  (bind _my_character (Variables|Default|GetMy%20Character))
  (bind _pillar (Variables|Default|GetPillar))
  (bind _my_character_2 (Variables|Default|GetMy%20Character))
  (bind _pillar_2 (Variables|Default|GetPillar))
  (bind _returnvalue_5 (Transformation|GetActorLocation _pillar))
  (bind _returnvalue_6 (Transformation|GetActorLocation _my_character_2))
  (bind _returnvalue_7 (Transformation|GetActorLocation _pillar_2))
  (bind _returnvalue_8 (Transformation|GetActorLocation _my_character))
  (bind _returnvalue_9 (Math|Vector|Distance(Vector) _returnvalue_4 _returnvalue_8))
  (bind _returnvalue_10 (Math|Vector|Distance(Vector) _returnvalue _returnvalue_5))
  (bind _returnvalue_11 (<= _returnvalue_10 1e+02))
  (bind _returnvalue_12 (<= _returnvalue_9 1e+02))
  (Variables|Default|SetDelta%20Seconds DeltaSeconds)
  (bind _output_get (Variables|Default|SettoCloseToPillarAndToCharacter (and _returnvalue_12 _returnvalue_11)))
  (if (not _output_get)
    (if (Variables|Default|GetmoveToCharacter)
      (Transformation|SetActorLocationAndRotation (Math|Interpolation|VInterpTo _returnvalue_2 _returnvalue_6 (Variables|Default|GetDelta%20Seconds) 0.5) (Math|Rotator|FindLookatRotation _returnvalue_2 _returnvalue_6))
      (Variables|Default|SetmoveToCharacter (not _returnvalue_12))
      (else
        (Transformation|SetActorLocationAndRotation (Math|Interpolation|VInterpTo _returnvalue_3 _returnvalue_7 (Variables|Default|GetDelta%20Seconds) 0.5) (Math|Rotator|FindLookatRotation _returnvalue_3 _returnvalue_7))
        (Variables|Default|SetmoveToCharacter _returnvalue_11)))))

(fn ConstructionScript)