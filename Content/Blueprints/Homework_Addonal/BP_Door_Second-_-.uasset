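; BP_Door_Second is a sliding double door that opens when the player presses its linked switches in shuffled order before time runs out.
; BeginPlay filters and shuffles valid BP_Interactive_Switch instances, binds their press events and activates the first.
; The first press starts a countdown shown on a progress-bar widget; each press activates the next switch.
; The final press pauses the timer and plays the door Timeline, while timeout resets progress but keeps the order.
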(event Custom|SwitchPressed_Event
  (params (Self_Ref :type BP%20Interactive%20Switch%20Object%20Reference))
  (Utilities|FlowControl|Sequence
    (:then_0
      ;[0.3735 1 0.2551] Після натискання перемикача ми додаємо одиницю та порівнюємо з довжиною валідного масива. Якщо число меньше, то активується наступна кнопка, якщо число співпадає то зупиняємо таймер та відчиняємо двері
      (bind _result (Math|Integer|IncrementInt (Variables|Default|GetSwitchesAlredyPressed))
        (:%20%20
          (if (== _result (Variables|Default|GetValidInstanceLenght))
            (Utilities|Time|PauseTimerbyHandle (Variables|Default|GetTimerHandle))
            ;[0.2334 1 0.3969] Анімація відкривання дверей
            (bind _dooropenspeed (Timeline|Timeline Play)
              (:Update
                (Transformation|SetRelativeLocation (Variables|Default|GetSM_Door_Left) (Math|Vector|MakeVector _dooropenspeed 0.0 0.0) false false)
                (Transformation|SetRelativeLocation (Variables|Default|GetSM_Door_Right) (Math|Vector|MakeVector (* _dooropenspeed -1.0) 0.0 0.0) false false)))
            (else
              (Default|ActivateSwitch (Utilities|Array|Get(acopy) (Variables|Default|GetButtonsValid) (Variables|Default|GetSwitchesAlredyPressed))))))))
    (:then_1
      ;[0.07926 1 0.6636] Після активації першого перемикача єдиноразово встановлюємо таймер на івент скидання перемикача
      (Utilities|FlowControl|DoOnce false
        (:Completed
          (bind _returnvalue (Utilities|Time|SetTimerbyEvent (delegate Custom|Reseting) (Variables|Default|GetTimeToResetDoor)))
          (Variables|Default|SetTimerHandle _returnvalue)
          (Widget|SetVisibility (Variables|Default|GetWB_Widget) "Visible"))))))

(event Custom|Reseting
  ;[1 0.8473 0.1357] Якщо гравець не встиг, то скидаємо його прогресію. Потім скидуємо і деактивуємо всі кнопки. І тільки першу активуємо. Тим самим зберігаєм послідовнісь яка згенерувалась при створенні левелу
  (Variables|Default|SetSwitchesAlredyPressed 0)
  (for (_array_element _array_index) (Variables|Default|GetButtonsValid)
    (Default|ResetSwitch _array_element)
    (Default|DeactivateSwitch _array_element)
    (if (== _array_index 0)
      (Default|ActivateSwitch _array_element)
      (Widget|SetVisibility (Variables|Default|GetWB_Widget) "Hidden")))
  ;[0.07926 1 0.6636] Після активації першого перемикача єдиноразово встановлюємо таймер на івент скидання перемикача
  (Utilities|FlowControl|DoOnce false) ; enters at Reset
)

(event EventBeginPlay
  (bind _switchesalredypressed (Variables|Default|GetSwitchesAlredyPressed))
  (bind _buttonsvalid (Variables|Default|GetButtonsValid))
  (bind _output (Utilities|Array|Get(acopy) _buttonsvalid _switchesalredypressed))
  (Utilities|FlowControl|Sequence
    (:then_0
      ;[1 1 1] Все що стосуєтся віджета
      (bind _returnvalue (UserInterface|CreateWidget "/Game/Blueprints/Homework_Addonal/UI/WB_ButtonHolding.WB_ButtonHolding_C"))
      (bind _output_get (Variables|Default|SetWB_Widget _returnvalue))
      (Widget|SetVisibility _output_get "Hidden")
      (Variables|/Script/UMG.TextBlock|SetText (Variables|/Game/Blueprints/Homework_Addonal/UI/WB_ButtonHolding.WB_ButtonHolding_C|GetTextBlock_226 (Variables|Default|GetWB_Widget)) "Time Left")
      (UserInterface|SetWidget (Variables|Default|GetWidget) (Variables|Default|GetWB_Widget))
      (Class|ProgressBar|SetFillColorandOpacity (Variables|/Game/Blueprints/Homework_Addonal/UI/WB_ButtonHolding.WB_ButtonHolding_C|GetProgressBar_0 (Variables|Default|GetWB_Widget)) "(R=1.000000,G=0.000000,B=0.086574,A=1.000000)"))
    (:then_1
      (Utilities|FlowControl|Delay 0.5) ; Затримка обробки
      ;[1 1 1] Перебироємо масив та записуємо в другий масив тількі валідні перемикачі. Також всі їх деактивуємо і для кожного валідного перемикача біндимо івент Switch Pressed
      (for _array_element (Variables|Default|GetButtonsInstance)
        (bind _asbp_interactive_switch (Utilities|Casting|CastToBP_Interactive_Switch _array_element))
        (Utilities|Array|Add (Variables|Default|GetButtonsValid) _asbp_interactive_switch)
        (Default|DeactivateSwitch _asbp_interactive_switch)
        (EventDispatchers|AssignSwitchPressed _asbp_interactive_switch (delegate Custom|SwitchPressed_Event)) ; З івент діспатчера перемикача
      )
      ;[0.237 1 0.9402] Після закінчення перебирання перетасовуємо масив валідних перемикачів та активуємо перший він же нульовий елемент
      (Utilities|Array|Shuffle _buttonsvalid)
      (Variables|Default|SetValidInstanceLenght (Utilities|Array|Length _buttonsvalid))
      (Utilities|IsValid _output
        (:Is%20Valid
          (Default|ActivateSwitch _output))))))

(event EventTick
  (params (DeltaSeconds :type Float%20%28single-precision%29))
  ;[1 1 1] Все що стосуєтся віджета
  (Variables|/Game/Blueprints/Homework_Addonal/UI/WB_ButtonHolding.WB_ButtonHolding_C|SetProcentage (Variables|Default|GetWB_Widget) (/ (Utilities|Time|GetTimerRemainingTimebyHandle (Variables|Default|GetTimerHandle)) (Variables|Default|GetTimeToResetDoor))))

(fn ConstructionScript)