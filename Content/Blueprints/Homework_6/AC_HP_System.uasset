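; Health component that tracks its owner's HP through the owner's any-damage event, with negative damage acting as healing.
; Damage passes through a Gate, gets clamped between zero and max, then fires health-change and, at zero, death notifications.
; OnShield closes the Gate, blocking damage and healing, and plays a supplied Niagara effect on BP_ThirdPersonCharacter.
; A retriggerable delay reopens the Gate and deactivates the effect.
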(event Custom|OnAnyDamage
  (params (DamagedActor :type Actor%20Object%20Reference) (Damage :type Float%20%28single-precision%29) (DamageType :type Damage%20Type%20Object%20Reference) (InstigatedBy :type Controller%20Object%20Reference) (DamageCauser :type Actor%20Object%20Reference))
  ;[1 1 1] Блокування пошкождення і лікування
  (Utilities|FlowControl|Gate false
    (:Exit
      (bind _output_get (Variables|Default|SetHealth (Math|Float|Clamp(Float) (- (Variables|Default|GetHealth) Damage) 0.0 (Variables|Default|GetMaxHealth))))
      (Default|CallOnChangeHealth)
      (if (== _output_get 0.0)
        (Default|CallOnDeath)))))

(event Custom|OnShield
  (params (ShieldTime :type Float%20%28double-precision%29) (NewParam :type Niagara%20System%20Object%20Reference))
  ;[1 1 1] Блокування пошкождення і лікування
  (Utilities|FlowControl|Sequence
    (:then_0
      (Utilities|FlowControl|Gate false) ; enters at Close
    )
    (:then_1
      (Utilities|FlowControl|RetriggerableDelay ShieldTime)
      (Utilities|FlowControl|Sequence
        (:then_0
          (Utilities|FlowControl|Gate false) ; enters at Open
        )
        (:then_1
          ;[1 0.2187 0.7765] Уффф... не сама краща система активації ніагара та візуальної демонстрації активного еффекту (щита) на персонажі
          (Components|Activation|Deactivate (Variables|Default|GetNiagara)))))
    (:then_2
      (bind _asbp_third_person_character (Utilities|Casting|CastToBP_ThirdPersonCharacter (Components|GetOwner)))
      (bind _output_get (Variables|Default|SetNiagara (Variables|/Game/Blueprints/Defaults/BP_ThirdPersonCharacter.BP_ThirdPersonCharacter_C|GetNiagara _asbp_third_person_character)))
      (Class|NiagaraComponent|SetAsset _output_get NewParam false)
      (Components|Activation|Activate (Variables|Default|GetNiagara) false))))

(event EventBeginPlay
  (Variables|Default|SetHealth (Variables|Default|GetMaxHealth))
  (Default|CallOnChangeHealth)
  (EventDispatchers|BindEventtoOnTakeAnyDamage (Components|GetOwner) (delegate Custom|OnAnyDamage)))