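; Actor component that toggles its owning Character's body between the Manny and Quinn simple mannequin skeletal meshes.
; A single ChangeMesh_Event casts the owner to Character and does nothing if that fails.
; It then compares the current mesh asset to Quinn and swaps to Manny on a match, or to Quinn otherwise.
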(event Custom|ChangeMesh_Event
  (bind _ascharacter (Utilities|Casting|CastToCharacter (Components|GetOwner)))
  (Variables|Default|SetMesh (Variables|/Script/Engine.Character|GetMesh _ascharacter))
  (if (== (Components|SkeletalMesh|GetSkeletalMeshAsset (Variables|Default|GetMesh)) "/Game/Characters/Mannequins/Meshes/SKM_Quinn_Simple.SKM_Quinn_Simple")
    (Components|SkeletalMesh|SetSkeletalMeshAsset (Variables|Default|GetMesh) "/Game/Characters/Mannequins/Meshes/SKM_Manny_Simple.SKM_Manny_Simple")
    (else
      (Components|SkeletalMesh|SetSkeletalMeshAsset (Variables|Default|GetMesh) "/Game/Characters/Mannequins/Meshes/SKM_Quinn_Simple.SKM_Quinn_Simple"))))