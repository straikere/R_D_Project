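; Timed puzzle door that slides its two panels apart once every linked BP_Interactive_Switch has been pressed.
; The first press starts a countdown on a widget progress bar and deactivates all switches except the next one.
; Each press removes that switch, shuffles the rest and activates the last, creating a random chain.
; Finishing pauses the timer and plays the door Timeline, while timeout rebuilds the list, reactivates all switches and hides the widget.
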(event Custom|Reseting
  (bind _buttonsvalid (Variables|Default|GetButtonsValid))
  ;[0.1269 0.7475 1] Процес скидання. Чистим валідний масив, заново проганяєм валідні перемикачі, паралельно активуя їх та відключая ім ліхтар. Після закінчення перебірки масива заново встановлюємо довжину його, вимикаємо віджет та скидаєм Do Once
  (Utilities|Array|Clear (Variables|Default|GetButtonsValid))
  (for _array_element (Variables|Default|GetButtonsInstance)
    (bind _asbp_interactive_switch (Utilities|Casting|CastToBP_Interactive_Switch _array_element))
    (Utilities|Array|Add (Variables|Default|GetButtonsValid) _asbp_interactive_switch)
    (Default|ActivateSwitch _asbp_interactive_switch)
    (Rendering|SetVisibility (Variables|/Game/Blueprints/Homework_08_Addonal/BP_Interactive_Switch.BP_Interactive_Switch_C|GetLight _asbp_interactive_switch) false false))
  (Variables|Default|SetValidInstanceLenght (Utilities|Array|Length (Variables|Default|GetButtonsValid)))
  (Widget|SetVisibility (Variables|Default|GetWB_Widget) "Hidden")
  ;[1 1 1] При першій активації перемикача встановлюємо таймер та видимість віджета. перебираємо весь валідний масив та деактивуєм його окрім останнього індексу, тому як він в потрібному стані
  (Utilities|FlowControl|DoOnce false) ; enters at Reset
)

(event Custom|SwitchPressed_Event
  (params (Self_Ref :type BP%20Interactive%20Switch%20Object%20Reference))
  (bind _buttonsvalid (Variables|Default|GetButtonsValid))
  (bind _buttonsvalid_2 (Variables|Default|GetButtonsValid))
  (bind _buttonsvalid_3 (Variables|Default|GetButtonsValid))
  ;[0.9849 1 0.3474] З натиснутого перемикача беремо його референс та виключаем його з массива. Перемішуемо массив
  (Utilities|Array|RemoveIndex _buttonsvalid_2 (Utilities|Array|FindItem _buttonsvalid_2 Self_Ref))
  (Utilities|Array|Shuffle (Variables|Default|GetButtonsValid))
  (Utilities|FlowControl|Sequence
    (:then_0
      ;[0.3735 1 0.2551] Після натискання перемикача ми віднімаємо одиницю та порівнюємо з нулем. Якщо число не співпадає з нулем, то активується наступна кнопка з кінця массива, якщо число співпадає то зупиняємо таймер та відчиняємо двері
      (bind _result (Math|Integer|DecrementInt (Variables|Default|GetValidInstanceLenght))
        (:%20%20
          (if (== _result 0)
            (Utilities|Time|PauseTimerbyHandle (Variables|Default|GetTimerHandle))
            ;[0.2334 1 0.3969] Анімація відкривання дверей
            (bind _dooropenspeed (Timeline|Timeline Play)
              (:Update
                (Transformation|SetRelativeLocation (Variables|Default|GetSM_Door_Left) (Math|Vector|MakeVector _dooropenspeed 0.0 0.0) false false)
                (Transformation|SetRelativeLocation (Variables|Default|GetSM_Door_Right) (Math|Vector|MakeVector (* _dooropenspeed -1.0) 0.0 0.0) false false)))
            (else
              (Default|ActivateSwitch (Utilities|Array|Get(acopy) _buttonsvalid (Utilities|Array|LastIndex _buttonsvalid))))))))
    (:then_1
      ;[1 1 1] При першій активації перемикача встановлюємо таймер та видимість віджета. перебираємо весь валідний масив та деактивуєм його окрім останнього індексу, тому як він в потрібному стані
      (Utilities|FlowControl|DoOnce false
        (:Completed
          (bind _returnvalue (Utilities|Time|SetTimerbyEvent (delegate Custom|Reseting) (Variables|Default|GetTimeToResetDoor)))
          (Variables|Default|SetTimerHandle _returnvalue)
          (Widget|SetVisibility (Variables|Default|GetWB_Widget) "Visible")
          (for (_array_element _array_index) _buttonsvalid_3
            (if (!= _array_index (Utilities|Array|LastIndex _buttonsvalid_3))
              (Default|DeactivateSwitch _array_element))))))))

(event EventBeginPlay
  (Utilities|FlowControl|Sequence
    (:then_0
      ;[0.6432 0.5073 1] Все що стосуєтся 3D віджета
      (bind _returnvalue (UserInterface|CreateWidget "/Game/Blueprints/Homework_08_Addonal/UI/WB_ButtonHolding.WB_ButtonHolding_C"))
      (bind _output_get (Variables|Default|SetWB_Widget _returnvalue))
      (Widget|SetVisibility _output_get "Hidden")
      (Variables|/Script/UMG.TextBlock|SetText (Variables|/Game/Blueprints/Homework_08_Addonal/UI/WB_ButtonHolding.WB_ButtonHolding_C|GetTextBlock_226 (Variables|Default|GetWB_Widget)) "Time Left")
      (UserInterface|SetWidget (Variables|Default|GetWidget) (Variables|Default|GetWB_Widget))
      (Class|ProgressBar|SetFillColorandOpacity (Variables|/Game/Blueprints/Homework_08_Addonal/UI/WB_ButtonHolding.WB_ButtonHolding_C|GetProgressBar_0 (Variables|Default|GetWB_Widget)) "(R=1.000000,G=0.000000,B=0.086574,A=1.000000)"))
    (:then_1
      (Utilities|FlowControl|Delay 0.5) ; Затримка обробки
      ;[1 1 1] Перебироємо масив та записуємо в другий масив тількі валідні перемикачі. Також всі їх деактивуємо і для кожного валідного перемикача біндимо івент Switch Pressed
      (for _array_element (Variables|Default|GetButtonsInstance)
        (bind _asbp_interactive_switch (Utilities|Casting|CastToBP_Interactive_Switch _array_element))
        (Utilities|Array|Add (Variables|Default|GetButtonsValid) _asbp_interactive_switch)
        (Rendering|SetVisibility (Variables|/Game/Blueprints/Homework_08_Addonal/BP_Interactive_Switch.BP_Interactive_Switch_C|GetLight _asbp_interactive_switch) false false)
        (EventDispatchers|BindEventtoSwitchPressed _asbp_interactive_switch (delegate Custom|SwitchPressed_Event)))
      (Variables|Default|SetValidInstanceLenght (Utilities|Array|Length (Variables|Default|GetButtonsValid))))))

(event EventTick
  (params (DeltaSeconds :type Float%20%28single-precision%29))
  ;[0.6432 0.5073 1] Все що стосуєтся 3D віджета
  (Variables|/Game/Blueprints/Homework_08_Addonal/UI/WB_ButtonHolding.WB_ButtonHolding_C|SetProcentage (Variables|Default|GetWB_Widget) (/ (Utilities|Time|GetTimerRemainingTimebyHandle (Variables|Default|GetTimerHandle)) (Variables|Default|GetTimeToResetDoor))))

(fn ConstructionScript)