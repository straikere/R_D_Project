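; Player controller that owns the game's UI, creating a UI_Base root widget on BeginPlay and pushing screens onto it.
; In the L_Homework_9_FrontEnd level it shows a background and main menu; other levels switch to game-only input with a hidden cursor.
; The menu input action pushes the pause menu, and a Message.PlayerDeath gameplay message listener pushes the death screen.
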(event Input|EnhancedActionEvents|EnhancedInputActionIA_Menu
  (params (ActionValue :type Boolean) (ElapsedSeconds :type Float%20%28double-precision%29) (TriggeredSeconds :type Float%20%28double-precision%29) (InputAction :type Input%20Action%20Object%20Reference :default "/Game/Blueprints/Homework_09/Input/IA_Menu.IA_Menu"))
  (:Started
    (Default|PushWidget (Variables|Default|GetUI_Base_Ref) "/Game/Blueprints/Homework_09/UI/UI_PauseMenu.UI_PauseMenu_C")))

(event EventBeginPlay
  (bind _self self)
  (bind _returnvalue (UserInterface|CreateWidget "/Game/Blueprints/Homework_09/UI/UI_Base.UI_Base_C" self))
  (bind _output_get (Variables|Default|SetUI_Base_Ref _returnvalue))
  (UserInterface|Viewport|AddtoViewport _output_get 0)
  (|ListenforGameplayMessages "(TagName=\"Message.PlayerDeath\")" "/Game/Blueprints/Defaults/MS_PlayerHealth.MS_PlayerHealth" "ExactMatch"
    (:then
      (bind _returnvalue_2 (Game|GetCurrentLevelName true))
      (if (== _returnvalue_2 "L_Homework_9_FrontEnd")
        (Default|PushHUDWidget (Variables|Default|GetUI_Base_Ref) "/Game/Blueprints/Homework_09/UI/UI_ImageBackground.UI_ImageBackground_C")
        (Default|PushWidget (Variables|Default|GetUI_Base_Ref) "/Game/Blueprints/Homework_09/UI/UI_MainMenu.UI_MainMenu_C")
        (else
          (Input|SetInputModeGameOnly _self false)
          (Variables|/Script/Engine.PlayerController|SetbShowMouseCursor _self false))))
    (:OnMessageReceived
      (Default|PushWidget (Variables|Default|GetUI_Base_Ref) "/Game/Blueprints/Homework_09/UI/UI_PlayerDeath.UI_PlayerDeath_C"))))

(fn ConstructionScript)