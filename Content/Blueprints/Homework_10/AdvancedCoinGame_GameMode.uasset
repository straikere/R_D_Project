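; Game mode for a timed coin-collection game that broadcasts win and lose messages.
; ChekCoins counts Coin-tagged actors as the target and notifies the UI.
; The first coin message starts the countdown and a per-second UI update; every coin restarts the countdown with two extra seconds.
; All communication uses GameplayMessageSubsystem channels, with collecting every coin winning and timer expiry losing.
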(event Custom|ChekCoins
  ;[0.9926 0.7157 1] Збір інформації про монетки. Їх кількість, та вивід Coin UI
  (bind _outactors (Actor|GetAllActorswithTag "Coin"))
  (bind _output_get (Variables|Default|SetValidCons (Utilities|Array|Length _outactors)))
  (Development|PrintString (Utilities|String|ToString(Integer) _output_get))
  (Messaging|BroadcastMessage (Subsystems|GetGameplayMessageSubsystem) "(TagName=\"UI.Coins\")" (Utilities|Struct|MakeMS_NullStructure true)))

(event Custom|YouLose
  ;[1 0.1705 0.2703] Якщо таймер вичерпано, то відправляем на виклик UI PlayerLose
  (Messaging|BroadcastMessage (Subsystems|GetGameplayMessageSubsystem) "(TagName=\"Message.PlayerLose\")" (Utilities|Struct|MakeMS_NullStructure true)))

(event Custom|SendTime
  ;[1 0.5344 0.3733] Система оновлення таймера в віджеті. Встановлюєтся один раз. Та кожну секунду відправляє данні про таймер та коїни в віджет
  (Messaging|BroadcastMessage (Subsystems|GetGameplayMessageSubsystem) "(TagName=\"UI.Coins\")" (Utilities|Struct|MakeMS_Coins (Variables|Default|GetCurrentCoinsColected) (Variables|Default|GetValidCons) (Math|Float|Round (Utilities|Time|GetTimerRemainingTimebyHandle (Variables|Default|GetTimer))))))

(event EventBeginPlay
  ;[1 1 1] Слухаємо монетки на їх збір
  (|ListenforGameplayMessages "(TagName=\"Message.CoinColected\")" "/Game/Blueprints/Defaults/MS_PlayerHealth.MS_PlayerHealth" "ExactMatch"
    (:OnMessageReceived
      ;[0.5483 1 0.2361] Додаємо до таймера 2 секунди тим що записуємо поточне значення в змінну + 2 секунди, та встановлюємо новий з новим часом
      (Utilities|FlowControl|Sequence
        (:then_0
          ;[1 1 1] Єдиноразово встановлюємо перший таймер на івент програшу
          (Utilities|FlowControl|DoOnce false
            (:Completed
              (bind _returnvalue (Utilities|Time|SetTimerbyEvent (delegate Custom|YouLose) (Variables|Default|GetTimeToCollect)))
              (Variables|Default|SetTimer _returnvalue)
              ;[1 0.5344 0.3733] Система оновлення таймера в віджеті. Встановлюєтся один раз. Та кожну секунду відправляє данні про таймер та коїни в віджет
              (Utilities|Time|SetTimerbyEvent (delegate Custom|SendTime) 1.0 true))))
        (:then_1
          (Variables|Default|SetTimeToCollect (+ (Utilities|Time|GetTimerRemainingTimebyHandle (Variables|Default|GetTimer)) 2.0))
          (Utilities|Time|ClearandInvalidateTimerbyHandle (Variables|Default|GetTimer))
          (bind _returnvalue_2 (Utilities|Time|SetTimerbyEvent (delegate Custom|YouLose) (Variables|Default|GetTimeToCollect)))
          (Variables|Default|SetTimer _returnvalue_2)
          ;[0.8334 0.4463 1] Додаємо коїн в Colected, та перевіряємо чи співпадає Colected з Valid Coins. Якщо не співпадає, примусово оновлюємо таймер, та данні про зібрані монетки
          (Math|Integer|IncrementInt (Variables|Default|GetCurrentCoinsColected)
            (:%20%20
              (if (== (Variables|Default|GetCurrentCoinsColected) (Variables|Default|GetValidCons))
                ;[0.8265 1 0.4931] Якщо перемога, зупиняем таймер, та викликаєм UI PlayerWin
                (Utilities|Time|ClearandInvalidateTimerbyHandle (Variables|Default|GetTimer))
                (Messaging|BroadcastMessage (Subsystems|GetGameplayMessageSubsystem) "(TagName=\"Message.PlayerWin\")" (Utilities|Struct|MakeMS_NullStructure true))
                (else
                  (CallFunction|SendTime)
                  ;[0.3441 1 0.7764] Debug
                  (Development|PrintString (Utilities|String|Append (Utilities|String|ToString(Integer) (- (Variables|Default|GetValidCons) (Variables|Default|GetCurrentCoinsColected))) " left coin")))))))))))

(fn ConstructionScript)