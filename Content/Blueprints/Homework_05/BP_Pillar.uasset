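; BP_Pillar is a pillar actor that spawns a BP_PillarFollower when it is hit.
; On hit, it destroys the previous follower and spawns a new one midway between itself and a BP_ThirdPersonCharacter, passing both to it.
; If the hitting actor is not that character, it prints a cast failure instead of spawning.
; A Gate closes after each handled hit and reopens after a short delay to throttle repeated hits.
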(event Custom|OnActorHit_Event
  (params (SelfActor :type Actor%20Object%20Reference) (OtherActor :type Actor%20Object%20Reference) (NormalImpulse :type Vector) (Hit :type Hit%20Result%20Structure%20%28by%20ref%29))
  (Utilities|FlowControl|Gate false :!label _label
    (:Exit
      (Utilities|IsValid (stale _follower)
        (:Is%20Valid
          (Actor|DestroyActor (stale _follower)))
        (:Is%20Not%20Valid
          _))
      (bind _follower (CallFunction|SpawnFollower SelfActor OtherActor))
      (Utilities|FlowControl|Sequence
        (:then_0
          (goto _label Close))
        (:then_1
          (Utilities|FlowControl|Delay 1.0)
          (goto _label Open))))))

(event EventBeginPlay
  (Collision|AssignOnActorHit (delegate Custom|OnActorHit_Event)))

(fn ConstructionScript)

(fn SpawnFollower
  (params (Pillar%20Actor :type Actor%20Object%20Reference) (Character%20Actror :type Actor%20Object%20Reference))
  (LocalVariables|SetPillar Pillar%20Actor)
  (bind _output_get (LocalVariables|SetCharacter Character%20Actror))
  (bind _asbp_third_person_character (Utilities|Casting|CastToBP_ThirdPersonCharacter _output_get)
    (:then
      (bind _returnvalue (Game|SpawnActorfromClass "/Game/Blueprints/Homework_04/BP_PillarFollower.BP_PillarFollower_C" (Math|Conversions|ToTransform(Vector) (/ (+ (Transformation|GetActorLocation (LocalVariables|GetPillar)) (Transformation|GetActorLocation (LocalVariables|GetCharacter))) 2)) "Undefined" "MultiplyWithRoot" 0 _asbp_third_person_character (LocalVariables|GetPillar) 0))
      (return _returnvalue))
    (:CastFailed
      (Development|PrintString "Cast failed"))))