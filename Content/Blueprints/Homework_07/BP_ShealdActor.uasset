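; BP_ShealdActor is a shield pickup that grants a timed shield to the actor that overlaps it.
; On BeginPlay it rolls a random shield duration, binds its overlap event and shows the duration on a text render as debug info.
; On overlap it passes the duration and shield effect to OnShield on the other actor's AC_HP_System component, then destroys itself.
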(event Custom|OnActorBeginOverlap_Event
  (params (OverlappedActor :type Actor%20Object%20Reference) (OtherActor :type Actor%20Object%20Reference))
  (Default|OnShield (Actor|GetComponentbyClass OtherActor "/Game/Blueprints/Homework_07/AC_HP_System.AC_HP_System_C") (Variables|Default|GetShieldTime) (Variables|Default|GetShieldEffect))
  (Actor|DestroyActor))

(event EventBeginPlay
  (Variables|Default|SetShieldTime (Math|Random|RandomFloatinRange 0.5 1.5))
  (EventDispatchers|AssignOnActorBeginOverlap (delegate Custom|OnActorBeginOverlap_Event))
  ;[1 1 1] Дебаг інформація
  (Rendering|Components|TextRender|SetText (Variables|Default|GetTextRender) (Utilities|Text|ToText(Float) (Variables|Default|GetShieldTime) "HalfToEven" false true 1 324 0 2)))

(fn ConstructionScript)