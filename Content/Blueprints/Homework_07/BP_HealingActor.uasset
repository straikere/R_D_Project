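; BP_HealingActor is a single-use pickup that heals the actor overlapping it by a random amount.
; On BeginPlay it rolls a random whole-number heal value, binds its begin-overlap event and shows the value on a text render as debug info.
; On overlap it applies the value as negative environmental damage to the other actor, without filtering, then destroys itself.
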(event Custom|OnActorBeginOverlap_Event
  (params (OverlappedActor :type Actor%20Object%20Reference) (OtherActor :type Actor%20Object%20Reference))
  (Game|Damage|ApplyDamage OtherActor (* (Variables|Default|GetBase%20Heal) -1.0) 0 0 "/Engine/EngineDamageTypes/DmgTypeBP_Environmental.DmgTypeBP_Environmental_C")
  (Actor|DestroyActor))

(event EventBeginPlay
  (Variables|Default|SetBase%20Heal (Math|Conversions|ToFloat(Integer) (Math|Random|RandomIntegerinRange 1 100)))
  (EventDispatchers|AssignOnActorBeginOverlap (delegate Custom|OnActorBeginOverlap_Event))
  ;[1 1 1] Дебаг інформація
  (Rendering|Components|TextRender|SetText (Variables|Default|GetTextRender) (Utilities|Text|ToText(Float) (Variables|Default|GetBase%20Heal) "HalfToEven")))

(fn ConstructionScript)