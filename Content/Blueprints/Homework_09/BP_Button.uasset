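; BP_Button is an interactable button actor that switches its sphere between two materials when the player presses Interact nearby.
; A box trigger enables input when the third-person character enters and disables it on exit, toggling a widget that starts hidden.
; While input is enabled, a FlipFlop on IA_Interact alternates the sphere's material on each press.
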(event OnComponentBeginOverlap(Box)
  (params (OverlappedComponent :type Primitive%20Component%20Object%20Reference) (OtherActor :type Actor%20Object%20Reference) (OtherComp :type Primitive%20Component%20Object%20Reference) (OtherBodyIndex :type Integer) (bFromSweep :type Boolean) (SweepResult :type Hit%20Result%20Structure%20%28by%20ref%29))
  (Utilities|Casting|CastToBP_ThirdPersonCharacter OtherActor)
  (Input|EnableInput (Game|GetPlayerController 0))
  (Rendering|ToggleVisibility (Variables|Default|GetWidget) false))

(event OnComponentEndOverlap(Box)
  (params (OverlappedComponent :type Primitive%20Component%20Object%20Reference) (OtherActor :type Actor%20Object%20Reference) (OtherComp :type Primitive%20Component%20Object%20Reference) (OtherBodyIndex :type Integer))
  (Utilities|Casting|CastToBP_ThirdPersonCharacter OtherActor)
  (Input|DisableInput (Game|GetPlayerController 0))
  (Rendering|ToggleVisibility (Variables|Default|GetWidget) false))

(event Input|EnhancedActionEvents|EnhancedInputActionIA_Interact
  (params (ActionValue :type Boolean) (ElapsedSeconds :type Float%20%28double-precision%29) (TriggeredSeconds :type Float%20%28double-precision%29) (InputAction :type Input%20Action%20Object%20Reference :default "/Game/Blueprints/Homework_08_Addonal/Input/IA_Interact.IA_Interact"))
  (bind _sphere (Variables|Default|GetSphere))
  (:Started
    (Utilities|FlowControl|FlipFlop
      (:A
        (Rendering|Material|SetMaterial _sphere 0 "/Engine/MapTemplates/Materials/BasicAsset03.BasicAsset03"))
      (:B
        (Rendering|Material|SetMaterial _sphere 0 "/Engine/MapTemplates/Materials/BasicAsset01.BasicAsset01")))))

(event EventBeginPlay
  (Rendering|SetVisibility (Variables|Default|GetWidget) false false))

(fn ConstructionScript)